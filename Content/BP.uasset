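; Blueprint that toggles an on-screen Slider widget with the F key.
; It creates the widget once at BeginPlay and keeps a reference to it.
; Tick polls the first player controller for F, and a FlipFlop alternates between showing and hiding.
; Showing adds the widget with the mouse cursor and Game and UI input, while hiding removes it and restores game-only input.
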(event `self.ReceiveBeginPlay`
  (bind _returnvalue (`|CreateWidget` "/Game/Slider.Slider_C"))
  (set `self.Slider REF` _returnvalue))

(event `self.ReceiveTick`
  (params (DeltaSeconds :type "Float (single-precision)"))
  (if (`PlayerController.WasInputKeyJustPressed` (`GameplayStatics.GetPlayerController` 0) "F")
    (`/Engine/EditorBlueprintResources/StandardMacros.FlipFlop`
      (:`A`
        (`self.Show Slider` self))
      (:`B`
        (`self.Hide Slider` self)))))

(fn `Hide Slider`
  (bind _returnvalue (`GameplayStatics.GetPlayerController` 0))
  (`Widget.RemoveFromParent` (`self.Slider REF`))
  (set `PlayerController.bShowMouseCursor` false _returnvalue)
  (`WidgetBlueprintLibrary.SetInputMode_GameOnly` _returnvalue)
  (return))

(fn `Show Slider`
  (bind _returnvalue (`GameplayStatics.GetPlayerController` 0))
  (bind _slider_ref (`self.Slider REF`))
  (`UserWidget.AddToViewport` _slider_ref 0)
  (set `PlayerController.bShowMouseCursor` true _returnvalue)
  (`WidgetBlueprintLibrary.SetInputMode_GameAndUIEx` _returnvalue _slider_ref)
  (return))

(fn `UserConstructionScript`)